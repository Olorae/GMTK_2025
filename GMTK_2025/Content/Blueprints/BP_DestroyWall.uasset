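; BP_DestroyWall is a wall actor that switches to a destroyed state when DestroyWallNow is called.
; The construction script sets the mesh to InitialMesh.
; DestroyWallNow runs once, swapping the mesh to NewMesh and hiding two decals.
; The Trigger overlap event is empty, so overlap alone does not start the destruction.
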(event OnComponentBeginOverlap(Trigger)
  (params (OverlappedComponent :type Primitive%20Component%20Object%20Reference) (OtherActor :type Actor%20Object%20Reference) (OtherComp :type Primitive%20Component%20Object%20Reference) (OtherBodyIndex :type Integer) (bFromSweep :type Boolean) (SweepResult :type Hit%20Result%20Structure%20%28by%20ref%29)))

(event Custom|DestroyWallNow
  (Utilities|FlowControl|DoOnce false
    (:Completed
      (Components|StaticMesh|SetStaticMesh (Variables|Default|GetMesh) (Variables|Default|GetNew%20Mesh))
      (Rendering|SetVisibility (Variables|Default|GetDecal) false false))))

(fn ConstructionScript
  (Components|StaticMesh|SetStaticMesh (Variables|Default|GetMesh) (Variables|Default|GetInitialMesh)))