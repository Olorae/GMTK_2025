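; BP_MouseTrap is a mouse trap hazard that reacts to the third-person character through two overlap boxes.
; Overlapping Box1 launches the SMTrapMouse component upward with a velocity-change impulse at its location.
; Overlapping Box triggers the same launch if the character's FatnessLVL is 2.
; Otherwise, Box applies damage to the character and prints a death message.
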(event OnComponentBeginOverlap(Box1)
  (params (OverlappedComponent :type Primitive%20Component%20Object%20Reference) (OtherActor :type Actor%20Object%20Reference) (OtherComp :type Primitive%20Component%20Object%20Reference) (OtherBodyIndex :type Integer) (bFromSweep :type Boolean) (SweepResult :type Hit%20Result%20Structure%20%28by%20ref%29))
  (bind _sm_trapmouse (Variables|Default|GetSM_TrapMouse))
  (Utilities|Casting|CastToBP_ThirdPersonCharacter OtherActor)
  (Class|PrimitiveComponent|AddVelocityChangeImpulseatLocation _sm_trapmouse "0.000000,0.000000,1000.000000" (Transformation|GetWorldLocation _sm_trapmouse) "None"))

(event OnComponentBeginOverlap(Box)
  (params (OverlappedComponent :type Primitive%20Component%20Object%20Reference) (OtherActor :type Actor%20Object%20Reference) (OtherComp :type Primitive%20Component%20Object%20Reference) (OtherBodyIndex :type Integer) (bFromSweep :type Boolean) (SweepResult :type Hit%20Result%20Structure%20%28by%20ref%29))
  (bind _sm_trapmouse (Variables|Default|GetSM_TrapMouse))
  (bind _asbp_third_person_character (Utilities|Casting|CastToBP_ThirdPersonCharacter OtherActor))
  (if (== (Variables|/Game/ThirdPerson/Blueprints/BP_ThirdPersonCharacter.BP_ThirdPersonCharacter_C|GetFatness%20LVL _asbp_third_person_character) 2)
    (Class|PrimitiveComponent|AddVelocityChangeImpulseatLocation _sm_trapmouse "0.000000,0.000000,1000.000000" (Transformation|GetWorldLocation _sm_trapmouse) "None")
    (else
      (Game|Damage|ApplyDamage _asbp_third_person_character 1.0 0 0)
      (Development|PrintString "DEATH!"))))

(event EventBeginPlay)

(event Collision|EventActorBeginOverlap
  (params (OtherActor :type Actor%20Object%20Reference)))

(event EventTick
  (params (DeltaSeconds :type Float%20%28single-precision%29)))

(fn ConstructionScript)