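; BP_CatPawn is a cat pawn built to sweep its yaw back and forth around its starting facing, though that motion is currently disconnected.
; BeginPlay stores the starting rotation and derives limits 90 degrees to either side.
; The unwired logic flips a turn-direction flag near either limit and eases toward the active one with RInterpTo.
; Tick is empty, so the pawn never rotates itself.
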(event EventBeginPlay
  (Variables|Default|SetStartingRotation (Transformation|GetActorRotation self))
  (Variables|Default|SetMaxRotation (Math|Rotator|MakeRotator (.roll (Variables|Default|GetStartingRotation)) (.pitch (Variables|Default|GetStartingRotation)) (+ (.yaw (Variables|Default|GetStartingRotation)) 9e+01)))
  (Variables|Default|SetMinRotation (Math|Rotator|MakeRotator (.roll (Variables|Default|GetStartingRotation)) (.pitch (Variables|Default|GetStartingRotation)) (- (.yaw (Variables|Default|GetStartingRotation)) 9e+01))))

(event Collision|EventActorBeginOverlap
  (params (OtherActor :type Actor%20Object%20Reference)))

(event EventTick
  (params (DeltaSeconds :type Float%20%28single-precision%29)))

(fn ConstructionScript)