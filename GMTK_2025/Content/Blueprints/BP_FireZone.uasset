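; BP_FireZone is a fire hazard that damages the player after enough continuous exposure.
; A timeline, rate-set by Speed and started from a configurable position, raises the hitbox and scales Niagara spawn rate and velocities together.
; While the third-person character overlaps, a fast looping timer accumulates exposure and audio plays.
; At TimeBeforeDeath it applies damage; leaving resets the count and stops the sound.
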(event OnComponentBeginOverlap(Hitbox)
  (params (OverlappedComponent :type Primitive%20Component%20Object%20Reference) (OtherActor :type Actor%20Object%20Reference) (OtherComp :type Primitive%20Component%20Object%20Reference) (OtherBodyIndex :type Integer) (bFromSweep :type Boolean) (SweepResult :type Hit%20Result%20Structure%20%28by%20ref%29))
  (Utilities|Casting|CastToBP_ThirdPersonCharacter OtherActor)
  (bind _returnvalue (Utilities|Time|SetTimerbyEvent (delegate Custom|StartTakingDMG) 0.001 true))
  (bind _returnvalue_2 (AddComponent|AddAudioComponent false))
  (Variables|Default|SetAudio%20Cooking _returnvalue_2))

(event OnComponentEndOverlap(Hitbox)
  (params (OverlappedComponent :type Primitive%20Component%20Object%20Reference) (OtherActor :type Actor%20Object%20Reference) (OtherComp :type Primitive%20Component%20Object%20Reference) (OtherBodyIndex :type Integer))
  (bind _audio_cooking (Variables|Default|GetAudio%20Cooking))
  (Utilities|Casting|CastToBP_ThirdPersonCharacter OtherActor)
  (Utilities|Time|ClearandInvalidateTimerbyHandle (stale OnComponentBeginOverlap(Hitbox) _returnvalue))
  (Variables|Default|SetFoundAmount 0.0)
  (Utilities|IsValid _audio_cooking
    (:Is%20Valid
      (Audio|Components|Audio|Stop _audio_cooking))))

(event Custom|StartTakingDMG
  (Variables|Default|SetFoundAmount (Math|Float|Clamp(Float) (+ 0.001 (Variables|Default|GetFoundAmount)) 0.0 (Variables|Default|GetTimeBeforeDeath)))
  (if (>= (Variables|Default|GetFoundAmount) (Variables|Default|GetTimeBeforeDeath))
    (bind _asbp_third_person_character (Utilities|Casting|CastToBP_ThirdPersonCharacter (Game|Player|GetPlayerPawn 0)))
    (Game|Damage|ApplyDamage _asbp_third_person_character 1.0 0 0)
    (Utilities|Time|ClearandInvalidateTimerbyHandle (stale OnComponentBeginOverlap(Hitbox) _returnvalue))
    (Development|PrintString "DEATH!")))

(event EventBeginPlay
  (bind _niagara (Variables|Default|GetNiagara))
  (Components|Timeline|SetPlaybackPosition (Variables|Default|GetTimelineAlpha) (Variables|Default|GetStart%20Position%20of%20timeline) false true)
  (bind _newtrack_0 (Timeline|TimelineAlpha Play)
    (:Update
      (Variables|Default|SetAlphaTimeline _newtrack_0)
      (Transformation|SetRelativeLocation (Variables|Default|GetHitbox) (Math|Vector|MakeVector 0.0 0.0 (Math|Float|Lerp -9.5e+02 -235.0 (Variables|Default|GetAlphaTimeline))) false false)
      (Niagara|SetNiagaraVariable(Float) (Variables|Default|GetNiagara) "SpawnRate" (Math|Float|Lerp 0.0 1.2e+02 (Variables|Default|GetAlphaTimeline)))
      (Utilities|FlowControl|Sequence
        (:then_0
          (Niagara|SetNiagaraVariable(Float) _niagara "Minimum_Velocity Speed" (Math|Float|Lerp 0.0 1.9e+03 (Variables|Default|GetAlphaTimeline)))
          (Niagara|SetNiagaraVariable(Float) _niagara "Maximum_Velocity Speed" (Math|Float|Lerp 0.0 2.6e+03 (Variables|Default|GetAlphaTimeline))))
        (:then_1
          (Niagara|SetNiagaraVariable(Float) _niagara "Minimum_Velocity SpeedFaster" (* (Math|Float|Lerp 0.0 1.9e+03 (Variables|Default|GetAlphaTimeline)) 1.1))
          (Niagara|SetNiagaraVariable(Float) _niagara "Maximum_Velocity SpeedFaster" (* (Math|Float|Lerp 0.0 2.6e+03 (Variables|Default|GetAlphaTimeline)) 1.1)))))))

(event Collision|EventActorBeginOverlap
  (params (OtherActor :type Actor%20Object%20Reference)))

(event EventTick
  (params (DeltaSeconds :type Float%20%28single-precision%29)))

(fn ConstructionScript
  (Components|Timeline|SetPlayRate (Variables|Default|GetTimelineAlpha) (Variables|Default|GetSpeed)))