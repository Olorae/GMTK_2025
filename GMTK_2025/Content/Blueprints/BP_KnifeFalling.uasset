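; Falling knife trap that drops when the third-person character enters its trigger and damages them on kill-zone contact.
; A one-shot overlap plays a speed-adjustable timeline intended to lerp the knife between two target heights, then move the kill zone away.
; A kill re-arms the trigger and returns the knife to its start height after the character's respawn delay.
; The construction script applies mesh, size and start height.
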(event OnComponentBeginOverlap(Trigger)
  (params (OverlappedComponent :type Primitive%20Component%20Object%20Reference) (OtherActor :type Actor%20Object%20Reference) (OtherComp :type Primitive%20Component%20Object%20Reference) (OtherBodyIndex :type Integer) (bFromSweep :type Boolean) (SweepResult :type Hit%20Result%20Structure%20%28by%20ref%29))
  (bind _fallingknife_timeline (Variables|Default|GetFallingKnife_Timeline))
  (Utilities|Casting|CastToBP_ThirdPersonCharacter OtherActor)
  (Utilities|FlowControl|DoOnce false
    (:Completed
      (Components|Timeline|SetPlayRate _fallingknife_timeline (Variables|Default|GetFallingSpeed))
      (Components|Timeline|PlayfromStart _fallingknife_timeline))))

(event OnComponentBeginOverlap(KillZone)
  (params (OverlappedComponent :type Primitive%20Component%20Object%20Reference) (OtherActor :type Actor%20Object%20Reference) (OtherComp :type Primitive%20Component%20Object%20Reference) (OtherBodyIndex :type Integer) (bFromSweep :type Boolean) (SweepResult :type Hit%20Result%20Structure%20%28by%20ref%29))
  (bind _fallingknife_timeline (Variables|Default|GetFallingKnife_Timeline))
  (bind _asbp_third_person_character (Utilities|Casting|CastToBP_ThirdPersonCharacter OtherActor))
  (Game|Damage|ApplyDamage _asbp_third_person_character 1.0 0 0)
  (Development|PrintString "DEATH!")
  (Utilities|FlowControl|Sequence
    (:then_0
      (Utilities|FlowControl|DoOnce false) ; enters at Reset
    )
    (:then_1
      (Utilities|FlowControl|Delay (Variables|/Game/ThirdPerson/Blueprints/BP_ThirdPersonCharacter.BP_ThirdPersonCharacter_C|GetTime%20Before%20Respawn _asbp_third_person_character))
      (Transformation|SetRelativeLocation (Variables|Default|GetKnifeEnd) (Math|Vector|MakeVector 0.0 0.0 (.z (Variables|Default|GetTarget01))) false false))))

(event EventBeginPlay)

(event Collision|EventActorBeginOverlap
  (params (OtherActor :type Actor%20Object%20Reference)))

(event EventTick
  (params (DeltaSeconds :type Float%20%28single-precision%29)))

(fn ConstructionScript
  (Transformation|SetRelativeLocation (Variables|Default|GetKnifeEnd) (Math|Vector|MakeVector 0.0 0.0 (.z (Variables|Default|GetTarget01))) false false)
  (Components|StaticMesh|SetStaticMesh (Variables|Default|GetSM_Knife01) (Variables|Default|GetKnife%20Mesh))
  (Transformation|SetRelativeScale3D (Variables|Default|GetKnifeEnd) (Math|Conversions|ToVector(Float) (Variables|Default|GetKnife%20Size))))