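; Checkpoint actor that records itself as LastCheckPoint in BP_MouseGameMode when the player character overlaps its Trigger, and can double as a cheese goal.
; IsCheese drives the construction script, which shows the cheese mesh, auto-activates Glow and sizes the Sphere, or zeroes its radius otherwise.
; Any Sphere overlap, after a delay, saves the checkpoint, raises fatness levels on game mode and player, then calls the player's RespawnFromWinCon.
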(event OnComponentBeginOverlap(Trigger)
  (params (OverlappedComponent :type Primitive%20Component%20Object%20Reference) (OtherActor :type Actor%20Object%20Reference) (OtherComp :type Primitive%20Component%20Object%20Reference) (OtherBodyIndex :type Integer) (bFromSweep :type Boolean) (SweepResult :type Hit%20Result%20Structure%20%28by%20ref%29))
  (Utilities|Casting|CastToBP_ThirdPersonCharacter OtherActor)
  (bind _asbp_mouse_game_mode (Utilities|Casting|CastToBP_MouseGameMode (Game|GetGameMode)))
  (Variables|/Game/Blueprints/BP_MouseGameMode.BP_MouseGameMode_C|SetLast%20CheckPoint _asbp_mouse_game_mode self)
  (Development|PrintString "CheckPoint!"))

(event OnComponentBeginOverlap(Sphere)
  (params (OverlappedComponent :type Primitive%20Component%20Object%20Reference) (OtherActor :type Actor%20Object%20Reference) (OtherComp :type Primitive%20Component%20Object%20Reference) (OtherBodyIndex :type Integer) (bFromSweep :type Boolean) (SweepResult :type Hit%20Result%20Structure%20%28by%20ref%29))
  (Development|PrintString "Got Cheese!")
  (Utilities|FlowControl|Delay 2.0)
  (bind _asbp_mouse_game_mode (Utilities|Casting|CastToBP_MouseGameMode (Game|GetGameMode)))
  (Variables|/Game/Blueprints/BP_MouseGameMode.BP_MouseGameMode_C|SetLast%20CheckPoint _asbp_mouse_game_mode self)
  (Development|PrintString "CheckPoint!")
  ;[1 1 1] Increase Level Chunk
  (bind _asbp_mouse_game_mode_2 (Utilities|Casting|CastToBP_MouseGameMode (Game|GetGameMode)))
  (Default|IncreaseFatLVL _asbp_mouse_game_mode_2)
  ;[1 1 1] increase player chunk
  (bind _asbp_third_person_character (Utilities|Casting|CastToBP_ThirdPersonCharacter (Game|Player|GetPlayerPawn 0)))
  (Default|IncreaseFatnessLVL _asbp_third_person_character)
  (Default|RespawnfromWinCon _asbp_third_person_character))

(event EventBeginPlay)

(event Collision|EventActorBeginOverlap
  (params (OtherActor :type Actor%20Object%20Reference)))

(event EventTick
  (params (DeltaSeconds :type Float%20%28single-precision%29)))

(fn ConstructionScript
  (bind _sphere (Variables|Default|GetSphere))
  (if (Variables|Default|GetIsCheese)
    (Components|Sphere|SetSphereRadius _sphere 480.541565 true)
    (Rendering|SetVisibility (Variables|Default|GetSM_Cheese) true false)
    (Components|Activation|SetAutoActivate (Variables|Default|GetGlow) true)
    (else
      (Components|Sphere|SetSphereRadius _sphere 0.0 true)
      (Rendering|SetVisibility (Variables|Default|GetSM_Cheese) false false)
      (Components|Activation|SetAutoActivate (Variables|Default|GetGlow) false))))