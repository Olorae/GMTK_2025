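; BP_CatRobot is a robot actor with a vision cone that checks its line of sight to the player character.
; When BP_ThirdPersonCharacter enters the cone, a fast looping timer sphere-traces from EyeZone to the character's mesh on the Camera channel.
; The trace only draws debug and prints the hit actor's name; any end overlap on the cone clears the timer.
; An AlphaRotation timeline exists but is never triggered.
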(event OnComponentBeginOverlap(Cone)
  (params (OverlappedComponent :type Primitive%20Component%20Object%20Reference) (OtherActor :type Actor%20Object%20Reference) (OtherComp :type Primitive%20Component%20Object%20Reference) (OtherBodyIndex :type Integer) (bFromSweep :type Boolean) (SweepResult :type Hit%20Result%20Structure%20%28by%20ref%29))
  (bind _asbp_third_person_character (Utilities|Casting|CastToBP_ThirdPersonCharacter OtherActor))
  (Variables|Default|SetAs%20BP%20Third%20Person%20Character _asbp_third_person_character)
  (Variables|Default|GetAs%20BP%20Third%20Person%20Character
    (:then
      (CallFunction|StartLineTrace))
    (:else)))

(event OnComponentEndOverlap(Cone)
  (params (OverlappedComponent :type Primitive%20Component%20Object%20Reference) (OtherActor :type Actor%20Object%20Reference) (OtherComp :type Primitive%20Component%20Object%20Reference) (OtherBodyIndex :type Integer))
  (Utilities|Time|ClearandInvalidateTimerbyHandle (stale Custom|Start%20Line%20Trace _returnvalue)))

(event Custom|Start%20Line%20Trace
  (bind _returnvalue (Utilities|Time|SetTimerbyEvent (delegate Custom|Searching) 0.001 true)))

(event Custom|Searching
  (bind _outhit (Collision|SphereTraceByChannel (Transformation|GetWorldLocation (Variables|Default|GetEyeZone)) (Transformation|GetWorldLocation (Variables|/Script/Engine.Character|GetMesh (Variables|Default|GetAs%20BP%20Third%20Person%20Character))) 1.0 "TraceTypeQuery2" false 0 "ForOneFrame"))
  (Development|PrintString (Utilities|GetDisplayName (.HitActor (Collision|BreakHitResult _outhit))) true true "(R=0.000000,G=0.660000,B=1.000000,A=1.000000)" 2.0 "eaaa"))

(event EventBeginPlay)

(event Collision|EventActorBeginOverlap
  (params (OtherActor :type Actor%20Object%20Reference)))

(event EventTick
  (params (DeltaSeconds :type Float%20%28single-precision%29)))

(fn ConstructionScript)