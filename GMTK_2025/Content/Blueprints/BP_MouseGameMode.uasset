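; Game mode for a mouse game that handles pausing, checkpoint respawns and fatness-based level progression.
; RespawnPlayer teleports the existing character to LastCheckPoint with a yaw offset, or to a hard-coded fallback location.
; IncreaseFatLVL raises a clamped fatness level, streams in matching spawnable sublevels, and enables physics on pushable objects or mousetraps.
; The construction script sets shadow distance scale to zero by console command.
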(event Custom|Respawn%20Player
  (bind _asbp_third_person_character (Utilities|Casting|CastToBP_ThirdPersonCharacter (Game|Player|GetPlayerPawn 0)))
  (bind _last_checkpoint (Variables|Default|GetLast%20CheckPoint)
    (:then
      (Transformation|SetWorldTransform (Variables|/Script/Engine.Character|GetCapsuleComponent _asbp_third_person_character) (Math|Transform|MakeTransform (.location (Transformation|GetWorldTransform (Variables|/Game/Blueprints/BP_CheckPoint.BP_CheckPoint_C|GetPosition%20of%20Respawn _last_checkpoint))) (Math|Rotator|MakeRotator (.roll (.rotation (Transformation|GetWorldTransform (Variables|/Game/Blueprints/BP_CheckPoint.BP_CheckPoint_C|GetPosition%20of%20Respawn _last_checkpoint)))) (.pitch (.rotation (Transformation|GetWorldTransform (Variables|/Game/Blueprints/BP_CheckPoint.BP_CheckPoint_C|GetPosition%20of%20Respawn _last_checkpoint)))) (+ (.yaw (.rotation (Transformation|GetWorldTransform (Variables|/Game/Blueprints/BP_CheckPoint.BP_CheckPoint_C|GetPosition%20of%20Respawn _last_checkpoint)))) 9e+01)) "1.000000,1.000000,1.000000") false true))
    (:else
      ;[1 1 1] no Checkpoint??
      (Transformation|SetWorldTransform (Variables|/Script/Engine.Character|GetCapsuleComponent _asbp_third_person_character) (Math|Transform|MakeTransform "1365.000000,-279.000000,497.000000" "0, 0, 0" "1.000000,1.000000,1.000000") false true)
      (Development|PrintString "respawn w no checkpoint"))))

(event Custom|IncreaseFatLVL
  (Variables|Default|SetFatness%20Level (Math|Integer|Clamp(Integer) (+ (Variables|Default|GetFatness%20Level) 1) 0 2))
  (Utilities|FlowControl|Sequence
    (:then_0
      ;[1 1 1] LVL 2 Fatness obstacles
      (if (== (Variables|Default|GetFatness%20Level) 0)
        (Game|LoadStreamLevel(byName) "SLVL_S01_Spawnables" true)))
    (:then_1
      ;[1 1 1] LVL 2 Fatness obstacles
      (if (== (Variables|Default|GetFatness%20Level) 1)
        (Game|LoadStreamLevel(byName) "SLVL_S02_Spawnables" true)
        (bind _outactors (Actor|GetAllActorsOfClass "/Game/Blueprints/BP_PushableObject.BP_PushableObject_C"))
        (for _array_element _outactors
          (Physics|SetSimulatePhysics (Variables|/Game/Blueprints/BP_PushableObject.BP_PushableObject_C|GetObject _array_element) true)
          (Class|PrimitiveComponent|SetLinearDamping (Variables|/Game/Blueprints/BP_PushableObject.BP_PushableObject_C|GetObject _array_element) 3.0))))
    (:then_2
      ;[1 1 1] LVL 3 Fatness obstacles
      (if (== (Variables|Default|GetFatness%20Level) 2)
        (Game|LoadStreamLevel(byName) "SLVL_S03_Spawnables" true)
        (bind _outactors_2 (Actor|GetAllActorsOfClass "/Game/Blueprints/BP_MouseTrap.BP_MouseTrap_C"))
        (for _array_element_2 _outactors_2
          (Physics|SetSimulatePhysics (Variables|/Game/Blueprints/BP_MouseTrap.BP_MouseTrap_C|GetSM_TrapMouse _array_element_2) true))))))

(event Custom|Pause%20Game
  (Game|SetGamePaused true))

(event Custom|UnPause%20Game
  (Game|SetGamePaused false))

(event EventBeginPlay
  (bind _asbp_game_instance (Utilities|Casting|CastToBP_GameInstance (Game|GetGameInstance)))
  (Variables|Default|SetBP_GameInstance _asbp_game_instance))

(event EventTick
  (params (DeltaSeconds :type Float%20%28single-precision%29)))

(fn ConstructionScript
  (Development|ExecuteConsoleCommand "r.Shadow.DistanceScale 0" 0))