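; Cheese win-condition checkpoint that advances the mouse game's fatness progression when its sphere is overlapped.
; A timeline started on BeginPlay bobs the cheese mesh up and down.
; After a short delay, overlap records this actor as the game mode's last checkpoint and raises its fat level.
; If the overlapping actor is the player character, it also gains fatness and respawns through RespawnFromWinCon.
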(event OnComponentBeginOverlap(Sphere_0)
  (params (OverlappedComponent :type Primitive%20Component%20Object%20Reference) (OtherActor :type Actor%20Object%20Reference) (OtherComp :type Primitive%20Component%20Object%20Reference) (OtherBodyIndex :type Integer) (bFromSweep :type Boolean) (SweepResult :type Hit%20Result%20Structure%20%28by%20ref%29))
  (Development|PrintString "Got Cheese!")
  (Utilities|FlowControl|Delay 2.0)
  (bind _asbp_mouse_game_mode (Utilities|Casting|CastToBP_MouseGameMode (Game|GetGameMode)))
  (Variables|/Game/Blueprints/BP_MouseGameMode.BP_MouseGameMode_C|SetLast%20CheckPoint _asbp_mouse_game_mode self)
  (Development|PrintString "CheckPoint!")
  ;[1 1 1] Increase Level Chunk
  (bind _asbp_mouse_game_mode_2 (Utilities|Casting|CastToBP_MouseGameMode (Game|GetGameMode)))
  (Default|IncreaseFatLVL _asbp_mouse_game_mode_2)
  ;[1 1 1] increase player chunk
  (bind _asbp_third_person_character (Utilities|Casting|CastToBP_ThirdPersonCharacter OtherActor))
  (Default|IncreaseFatnessLVL _asbp_third_person_character)
  (Default|RespawnfromWinCon _asbp_third_person_character))

(event EventBeginPlay
  (bind _up_and_down (Variables|Default|GetUp%20And%20down))
  (|CallParentFunction)
  (Components|Timeline|PlayfromStart _up_and_down)
  (Components|Timeline|SetPlayRate _up_and_down 1.5))

(event Collision|EventActorBeginOverlap
  (params (OtherActor :type Actor%20Object%20Reference))
  (|CallParentFunction OtherActor) ; This node is disabled and will not be called.\nDrag off pins to build functionality.
)

(event EventTick
  (params (DeltaSeconds :type Float%20%28single-precision%29))
  (|CallParentFunction DeltaSeconds) ; This node is disabled and will not be called.\nDrag off pins to build functionality.
)

(fn ConstructionScript
  (|CallParentFunction))